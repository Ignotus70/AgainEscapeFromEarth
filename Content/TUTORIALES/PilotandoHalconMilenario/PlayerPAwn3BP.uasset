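; Player character Blueprint in the PilotandoHalconMilenario tutorial, with forward movement, jumping and a speed-triggered ragdoll.
; The MoveForward axis feeds movement input along the actor's forward vector, and pressing the Jump action calls Jump.
; Tick checks the CharacterMovement velocity magnitude in any direction and enables physics simulation on all mesh bodies above a fixed threshold, with no logic to switch it back off.
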(event `InputAxis|MoveForward`
  (params (AxisValue :type "Float (single-precision)"))
  (`self.AddMovementInput` (`self.GetActorForwardVector`) AxisValue))

(event `InputAction|Jump`
  (params (Key :type "Key Structure"))
  (:`Pressed`
    (`self.Jump`)))

(event `self.ReceiveTick`
  (params (DeltaSeconds :type "Float (single-precision)"))
  (if (> (`KismetMathLibrary.VSize` (`MovementComponent.Velocity` (`self.CharacterMovement`))) 900.0)
    (`SkeletalMeshComponent.SetAllBodiesSimulatePhysics` (`self.Mesh`) true)))

(fn `UserConstructionScript`)