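; OceanPlanesBP is an ocean prop that tiles a plane mesh into a grid to form a large sea surface.
; Its construction script loops over NumPlanesX and NumPlanesY, adding one Hierarchical Instanced Static Mesh instance per cell at a fixed spacing.
; The event graph holds only disabled default events, so the actor has no runtime logic.
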(fn `UserConstructionScript`
  (for _index (range (`self.NumPlanesX`))
    (for _index_2 (range (`self.NumPlanesY`))
      (`InstancedStaticMeshComponent.AddInstance` (`self.HierarchicalInstancedStaticMesh`) (`KismetMathLibrary.MakeTransform` (`KismetMathLibrary.MakeVector` (* _index 25000.0) (* _index_2 25000.0)))))))