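; Flyable Millennium Falcon pawn that the player takes over when a ThirdPersonCharacter enters its sphere trigger, destroying that character.
; Power, Pitch and Yaw axes ease speed and turn rates with FInterpTo, with sharper yaw adding automatic banking roll.
; Tick applies those rates as local mesh rotation and forward actor movement.
; A dynamic material made in the construction script shows current power as a fraction of maximum speed.
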(event `self.ReceiveTick`
  (params (DeltaSeconds :type "Float (single-precision)"))
  (`SceneComponent.K2_AddLocalRotation` (`self.StaticMesh`) (`KismetMathLibrary.MakeRotator` (* (`self.RollActual`) DeltaSeconds) (* (`self.PitchActual`) DeltaSeconds) (* (`self.YawActual`) DeltaSeconds)) false false)
  (`self.K2_AddActorLocalOffset` (`KismetMathLibrary.MakeVector` (* DeltaSeconds (`self.VelocidadActual`)))))

(event `self.Sphere.OnComponentBeginOverlap`
  (params (OverlappedComponent :type "PrimitiveComponent Object Reference") (OtherActor :type "Actor Object Reference") (OtherComp :type "PrimitiveComponent Object Reference") (OtherBodyIndex :type Integer) (bFromSweep :type Boolean) (SweepResult :type "HitResult Structure (by ref)"))
  (bind _asthird_person_character (cast `/Game/ThirdPersonBP/Blueprints/ThirdPersonCharacter` OtherActor))
  (`Controller.Possess` (`GameplayStatics.GetPlayerController` 0) self)
  (`self.K2_DestroyActor` _asthird_person_character))

(event `InputAxis|Power`
  (params (AxisValue :type "Float (single-precision)"))
  (bind _output_get (set `self.VelocidadActual` (`KismetMathLibrary.FInterpTo` (`self.VelocidadActual`) (* AxisValue (`self.VelocidadMAX`)) (`GameplayStatics.GetWorldDeltaSeconds`) 20.0)))
  (`MaterialInstanceDynamic.SetScalarParameterValue` (`self.PowerMAT`) "PowerFactor" (/ _output_get (`self.VelocidadMAX`))))

(event `InputAxis|Pitch`
  (params (AxisValue :type "Float (single-precision)"))
  (set `self.PitchActual` (`KismetMathLibrary.FInterpTo` (`self.PitchActual`) (* AxisValue (`self.PitxhMAX`)) (`GameplayStatics.GetWorldDeltaSeconds`) 20.0)))

(event `InputAxis|Yaw`
  (params (AxisValue :type "Float (single-precision)"))
  (bind _output_get (set `self.YawActual` (`KismetMathLibrary.FInterpTo` (`self.YawActual`) (* AxisValue (`self.YawMAX`)) (`GameplayStatics.GetWorldDeltaSeconds`) 20.0)))
  (if (>= (`KismetMathLibrary.Abs` _output_get) 3.0)
    (set `self.RollActual` (`KismetMathLibrary.FInterpTo` (`self.RollActual`) _output_get (`GameplayStatics.GetWorldDeltaSeconds`) 10.0))
    (else
      (set `self.RollActual` (`KismetMathLibrary.FInterpTo` (`self.RollActual`) 0.0 (`GameplayStatics.GetWorldDeltaSeconds`) 10.0)))))

(fn `UserConstructionScript`
  (bind _returnvalue (`KismetMaterialLibrary.CreateDynamicMaterialInstance` "/Game/TUTORIALES/PilotandoHalconMilenario/Props/Falcon/PowerMAT.PowerMAT"))
  (bind _output_get (set `self.PowerMAT` _returnvalue))
  (`PrimitiveComponent.SetMaterial` (`self.StaticMesh`) 6 _output_get))