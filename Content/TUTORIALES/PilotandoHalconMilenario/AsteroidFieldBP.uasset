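; Asteroid field actor for a Millennium Falcon piloting tutorial that procedurally scatters NumAsteroids rocks within a sphere around itself.
; The Construction Script places each rock along a random direction at a distance up to DiamField, with random rotation, size and roughly 30% variation in proportions.
; All rocks are instances of one HierarchicalInstancedStaticMesh component, and the Event Graph holds no active logic.
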(fn `UserConstructionScript`
  (bind _returnvalue (`KismetMathLibrary.RandomFloatInRange` 0.3 8.0))
  (for _ (range (`self.NumAsteroids`))
    (`InstancedStaticMeshComponent.AddInstance` (`self.HierarchicalInstancedStaticMesh`) (`KismetMathLibrary.MakeTransform` (* (`KismetMathLibrary.RandomUnitVector`) (`KismetMathLibrary.RandomFloatInRange` 0.0 (`self.DiamField`))) (`KismetMathLibrary.RandomRotator` true) (+ (`KismetMathLibrary.MakeVector` _returnvalue _returnvalue _returnvalue) (* (`KismetMathLibrary.RandomUnitVector`) (* _returnvalue 0.3)))))))