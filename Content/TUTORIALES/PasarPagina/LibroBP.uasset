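; Book actor from a page-turn tutorial that renders text onto its page mesh at runtime.
; On BeginPlay it creates a Canvas Render Target and assigns a dynamic instance of MovPageMAT to the Pagina component.
; The target's update callback draws two text labels, feeds the texture into the material's LETRAS parameter and plays a timeline that animates the BrilloLetras brightness.
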(event `self.ReceiveBeginPlay`
  (bind _returnvalue (`CanvasRenderTarget2D.CreateCanvasRenderTarget2D` "/Script/Engine.CanvasRenderTarget2D" 512 512))
  (bind _output_get (set `self.TexturaPaginaMovimiento` _returnvalue))
  (add `CanvasRenderTarget2D.OnCanvasRenderTargetUpdate` _output_get (delegate `UpdatePage`))
  (bind _returnvalue_2 (`KismetMaterialLibrary.CreateDynamicMaterialInstance` "/Game/TUTORIALES/PasarPagina/MovPageMAT.MovPageMAT"))
  (bind _output_get_2 (set `self.DynMatPage` _returnvalue_2))
  (`PrimitiveComponent.SetMaterial` (`self.Pagina`) 0 _output_get_2)
  (`CanvasRenderTarget2D.UpdateResource` (`self.TexturaPaginaMovimiento`)))

(event `UpdatePage`
  (params (Canvas :type "Canvas Object Reference") (Width :type Integer) (Height :type Integer))
  (bind _dynmatpage (`self.DynMatPage`))
  (`Canvas.K2_DrawText` Canvas "/Game/TUTORIALES/PasarPagina/Myfont.Myfont" "Vertex \nAnimation \nTools" (0.0 0.0) (struct :`R` 1.0 :`G` 0.036361 :`A` 1.0) 0.0 (struct :`A` 1.0) (1.0 1.0) false false false (struct :`R` 1.0 :`G` 0.861831 :`A` 1.0))
  (`Canvas.K2_DrawText` Canvas "/Game/TUTORIALES/PasarPagina/Myfont.Myfont" "Canvas \nRender \nTarget" (256.0 0.0) (struct :`R` 1.0 :`G` 0.055031 :`A` 1.0) 0.0 (struct :`A` 1.0) (1.0 1.0) false false false (struct :`R` 1.0 :`G` 0.756678 :`A` 1.0))
  (`MaterialInstanceDynamic.SetTextureParameterValue` _dynmatpage "LETRAS" (`self.TexturaPaginaMovimiento`))
  (bind (_direction _brillo) (`Timeline|Timeline_0` :!via `PlayFromStart`)
    (:`Update`
      (`MaterialInstanceDynamic.SetScalarParameterValue` _dynmatpage "BrilloLetras" _brillo))))

(fn `UserConstructionScript`)